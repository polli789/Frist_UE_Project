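; BP_GM is the game mode that tracks elapsed time and the win or death outcome of a level.
; BeginPlay copies slow-time and jump settings from the game instance, applies jump hold time to BP_CHAR1, and adds audio.
; Win and die set Playerlive, then share an end-game path that pauses, shows the cursor and calls the HUD end screen.
; InPortal opens a level; truck-to-target AI and UI-only input nodes are unconnected.
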(event Custom|end%20game
  (Game|SetGamePaused true)
  (Variables|/Script/Engine.PlayerController|SetbShowMouseCursor (Game|GetPlayerController 0) true)
  (Default|EndGameHud (.AsHUD%20INGame (Utilities|Casting|CastToHUD_INGame (HUD|GetHUD (Game|GetPlayerController 0))))))

(event Custom|win
  (Variables|Default|SetPlayerlive true)
  (CallFunction|EndGame))

(event Custom|die
  (Variables|Default|SetPlayerlive false)
  (CallFunction|EndGame))

(event EventBeginPlay
  (bind _returnvalue (Game|GetGameInstance))
  (bind _isslow (Class|IFSLowTime|GetSlowTime(Message) _returnvalue))
  (Variables|Default|SetSlowTimeMode _isslow)
  (bind (_isjump _jumptime) (Class|IFJumpTime|GetJumpTime(Message) _returnvalue))
  (Variables|Default|SetIsJumpTime _isjump)
  (Variables|/Script/Engine.Character|SetJumpMaxHoldTime (.AsBP%20CHAR1 (Utilities|Casting|CastToBP_CHAR1 (Game|GetPlayerCharacter 0))) _jumptime)
  (AddComponent|AddAudioComponent false))

(event EventTick
  (params (DeltaSeconds :type Float%20%28single-precision%29))
  (Variables|Default|SetGM_Time (+ DeltaSeconds (Variables|Default|GetGM_Time))))

(fn ConstructionScript)

(fn InPortal
  (Game|OpenLevel(byObjectReference)))