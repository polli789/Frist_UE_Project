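; BP_Ins is a shared state holder, stored with the game mode Blueprints, for slow-time and time-jump status.
; SetSlowTime stores a slow-time flag, and SetJumpTime stores a jump flag with a JumpTime value.
; GetSlowTime and GetJumpTime return those stored values; the Blueprint itself applies no time effects.
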(event EventSetSlowTime
  (params (IsSlow :type Boolean))
  (Variables|Default|SetIsSlowTime IsSlow))

(event EventSetJumpTime
  (params (IsJump :type Boolean) (JumpTime :type Float%20%28double-precision%29))
  (Variables|Default|SetIsJumpTime IsJump)
  (Variables|Default|SetJumpTime JumpTime))

(fn GetJumpTime
  (return (Variables|Default|GetIsJumpTime) (Variables|Default|GetJumpTime)))

(fn GetSlowTime
  (return (Variables|Default|GetIsSlowTime)))